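; BP_Healthpack is a health pickup for the player that heals on contact or vanishes once passed.
; MeshCollision overlap heals BP_Player by calling DealDamage with the negated HealthPackHeal from GI_Instance, increments the collected pack count and destroys the actor.
; Ending overlap with PassingCollision also destroys it, removing packs the player leaves behind uncollected.
; The game instance reference is cached in the construction script.
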(event `self.MeshCollision.OnComponentBeginOverlap`
  (params (OverlappedComponent :type "PrimitiveComponent Object Reference") (OtherActor :type "Actor Object Reference") (OtherComp :type "PrimitiveComponent Object Reference") (OtherBodyIndex :type Integer) (bFromSweep :type Boolean) (SweepResult :type "HitResult Structure (by ref)"))
  (bind _asbp_player (cast `/Game/InfiniteMatrix/Blueprints/BP_Player` OtherActor))
  (`/Game/InfiniteMatrix/Blueprints/BP_Player.DealDamage` _asbp_player (- 0 (`/Game/InfiniteMatrix/Blueprints/GI_Instance.HealthPackHeal` (`self.GameInst`))))
  (`/Game/InfiniteMatrix/Blueprints/GI_Instance.IncreaseCollectedPackCount` (`self.GameInst`))
  (`self.K2_DestroyActor`))

(event `self.PassingCollision.OnComponentEndOverlap`
  (params (OverlappedComponent :type "PrimitiveComponent Object Reference") (OtherActor :type "Actor Object Reference") (OtherComp :type "PrimitiveComponent Object Reference") (OtherBodyIndex :type Integer))
  (cast `/Game/InfiniteMatrix/Blueprints/BP_Player` OtherActor)
  (`self.K2_DestroyActor`))

(fn `UserConstructionScript`
  (bind _asgi_instance (cast `/Game/InfiniteMatrix/Blueprints/GI_Instance` (`GameplayStatics.GetGameInstance`)))
  (set `self.GameInst` _asgi_instance))