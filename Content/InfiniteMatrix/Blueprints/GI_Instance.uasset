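; Game instance for InfiniteMatrix that keeps the run's score and gameplay statistics.
; Small functions add to Score or increment counters for passed and collided walls, collected packs, and collided and killed enemies.
; Reset zeroes every tally and turns off the ShowStatus flag.
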(fn `AddScore`
  (params (Delta :type Integer))
  (set `self.Score` (+ Delta (`self.Score`))))

(fn `IncreaseCollectedPackCount`
  (`/Engine/EditorBlueprintResources/StandardMacros.IncrementInt` (`self.CollectedPackCount`)))

(fn `IncreaseCollidedEnemyCount`
  (`/Engine/EditorBlueprintResources/StandardMacros.IncrementInt` (`self.CollidedEnemyCount`)))

(fn `IncreaseCollidedWallCount`
  (`/Engine/EditorBlueprintResources/StandardMacros.IncrementInt` (`self.CollidedWallCount`)))

(fn `IncreaseKilledEnemyCount`
  (`/Engine/EditorBlueprintResources/StandardMacros.IncrementInt` (`self.KilledEnemyCount`)))

(fn `IncreasePassedWallCount`
  (`/Engine/EditorBlueprintResources/StandardMacros.IncrementInt` (`self.PassedWallCount`)))

(fn `Reset`
  (set `self.Score` 0)
  (set `self.PassedWallCount` 0)
  (set `self.CollidedWallCount` 0)
  (set `self.CollectedPackCount` 0)
  (set `self.CollidedEnemyCount` 0)
  (set `self.KilledEnemyCount` 0)
  (set `self.ShowStatus` false))