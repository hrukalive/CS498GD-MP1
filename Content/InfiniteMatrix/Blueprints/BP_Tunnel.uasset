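; Tunnel segment for an endless tunnel game, with a rotating holed wall that damages the player and destroys projectiles.
; Tunnel and wall colors shift from green to red as health drops.
; The exit trigger rewards clean passes, asks the spawner for another segment, then destroys this one.
; Helpers randomize wall mesh and roll, and roll health pack and enemy spawns, placing them in shuffled cells within a polynomial-fitted radius.
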(event OnComponentBeginOverlap(TriggerZone)
  (params (OverlappedComponent :type Primitive%20Component%20Object%20Reference) (OtherActor :type Actor%20Object%20Reference) (OtherComp :type Primitive%20Component%20Object%20Reference) (OtherBodyIndex :type Integer) (bFromSweep :type Boolean) (SweepResult :type Hit%20Result%20Structure%20%28by%20ref%29))
  (bind _gameinst (Variables|Default|GetGameInst))
  (Utilities|Casting|CastToBP_Player OtherActor)
  (if (Variables|Default|GetHitWall)
    (Variables|Default|SetHitWall false)
    (else
      (Default|AddScore _gameinst (Variables|/Game/InfiniteMatrix/Blueprints/GI_Instance.GI_Instance_C|GetPassWallReward _gameinst))
      (Default|IncreasePassedWallCount _gameinst)))
  (Default|SpawnTunnelatSpawnPoint (Variables|Default|GetTunnelSpawner))
  (Actor|DestroyActor))

(event OnComponentBeginOverlap(WallMesh)
  (params (OverlappedComponent :type Primitive%20Component%20Object%20Reference) (OtherActor :type Actor%20Object%20Reference) (OtherComp :type Primitive%20Component%20Object%20Reference) (OtherBodyIndex :type Integer) (bFromSweep :type Boolean) (SweepResult :type Hit%20Result%20Structure%20%28by%20ref%29))
  (bind _gameinst (Variables|Default|GetGameInst))
  (bind _asbp_player (Utilities|Casting|CastToBP_Player OtherActor)
    (:then
      (bind _isdead (Default|IsDead _asbp_player))
      (if (not _isdead)
        (bind _isdead_2 (Default|DealDamage _asbp_player (Variables|/Game/InfiniteMatrix/Blueprints/GI_Instance.GI_Instance_C|GetWallCollisionDamage _gameinst)))
        (Default|IncreaseCollidedWallCount _gameinst)
        (Variables|Default|SetHitWall true)
        (if _isdead_2
          (Default|DisplayRestart _asbp_player))))
    (:CastFailed
      (bind _asbp_projectile (Utilities|Casting|CastToBP_Projectile OtherActor))
      (Actor|DestroyActor _asbp_projectile))))

(event EventBeginPlay
  (bind _asbp_player (Utilities|Casting|CastToBP_Player (Game|Player|GetPlayerPawn 0)))
  (Variables|Default|SetPlayer _asbp_player))

(event EventTick
  (params (DeltaSeconds :type Float%20%28single-precision%29))
  (bind _player (Variables|Default|GetPlayer))
  (bind _gameinst (Variables|Default|GetGameInst))
  (bind _staticmeshcomponent (Variables|Debug|GetStaticMeshComponent))
  (bind _health (Variables|/Game/InfiniteMatrix/Blueprints/BP_Player.BP_Player_C|GetHealth _player))
  (bind _maxhealth (Variables|/Game/InfiniteMatrix/Blueprints/GI_Instance.GI_Instance_C|GetMaxHealth _gameinst))
  (bind _returnvalue (Math|Conversions|ToFloat(Integer) _health))
  (bind _returnvalue_2 (Math|Conversions|ToFloat(Integer) _maxhealth))
  (bind _returnvalue_3 (|(min(1,(max(((2.500000*((MaxHealth-x)/MaxHealth))-1),0)))) _returnvalue_2 _returnvalue))
  (Transformation|AddLocalRotation (Variables|Default|GetWallMesh) (Math|Rotator|MakeRotator (* DeltaSeconds (Variables|Default|GetRotateSpeed)) 0.0 0.0) false false)
  ;[1 1 1] Tunnel color change with health
  (Rendering|Material|SetVectorParameterValueonMaterials _staticmeshcomponent "BackgroundColor" (Math|Vector|Lerp(Vector) (Math|Vector|MakeVector 0.0 0.06 0.007905) (Math|Vector|MakeVector 0.06 0.0 0.00081) _returnvalue_3))
  (Rendering|Material|SetVectorParameterValueonMaterials _staticmeshcomponent "TextColor" (Math|Vector|Lerp(Vector) (Math|Vector|MakeVector 0.0 1.0 0.286838) (Math|Vector|MakeVector 1.0 0.0 0.016063) _returnvalue_3))
  (Rendering|Material|SetVectorParameterValueonMaterials (Variables|Default|GetWallMesh) "Color" (Math|Vector|Lerp(Vector) (Math|Vector|MakeVector 0.0 1.0 0.286275) (Math|Vector|MakeVector 1.0 0.0934 0.0) _returnvalue_3)))

(fn ConstructionScript
  (bind _asgi_instance (Utilities|Casting|CastToGI_Instance (Game|GetGameInstance)))
  (Variables|Default|SetGameInst _asgi_instance))

(fn RandomizeWall
  (Components|StaticMesh|SetStaticMesh (Variables|Default|GetWallMesh) (Utilities|Select :Index (Math|Random|RandomIntegerinRange 0 3) :Option%200 "/Game/InfiniteMatrix/Meshes/SM_Hole_01.SM_Hole_01" :Option%201 "/Game/InfiniteMatrix/Meshes/SM_Hole_02.SM_Hole_02" :Option%202 "/Game/InfiniteMatrix/Meshes/SM_Hole_03.SM_Hole_03" :Option%203 "/Game/InfiniteMatrix/Meshes/SM_Hole_04.SM_Hole_04"))
  (Transformation|AddLocalRotation (Variables|Default|GetWallMesh) (Math|Rotator|MakeRotator (Math|Random|RandomFloatinRange 0.0 3.6e+02) 0.0 0.0) false false))

(fn RandomSpawnUtil
  (bind _loccellchoice (LocalVariables|GetLocCellChoice))
  (bind _output (Utilities|Array|Get(acopy) _loccellchoice))
  (bind _output_2 (Utilities|Array|Get(acopy) _loccellchoice 1))
  (bind _returnvalue (Math|Conversions|ToFloat(Integer) _output))
  (bind _returnvalue_2 (Math|Conversions|ToFloat(Integer) _output_2))
  (Utilities|FlowControl|Sequence
    (:then_0
      (bind _asgi_instance (Utilities|Casting|CastToGI_Instance (Game|GetGameInstance)))
      (LocalVariables|SetbSpawnHealthP:ack (== (Math|Random|RandomInteger (Math|Float|Ceil (/ 1.0 (Variables|/Game/InfiniteMatrix/Blueprints/GI_Instance.GI_Instance_C|GetEnemyProbability _asgi_instance)))) 0))
      (LocalVariables|SetbSpawnEnemy (== (Math|Random|RandomInteger (Math|Float|Ceil (/ 1.0 (Variables|/Game/InfiniteMatrix/Blueprints/GI_Instance.GI_Instance_C|GetHealthPackProbability _asgi_instance)))) 0)))
    (:then_1
      (Utilities|Array|Shuffle _loccellchoice)
      (return (|(vector((idx*100.000000),((r*percent)*(sin(angle))),((r*percent)*(cos(angle))))) _returnvalue (|(((((((1.606200*x)*x)*x)-((28.084101*x)*x))+(211.432495*x))-184.921097)-((((0.033463*x)*x)*x)*x)) _returnvalue) (Math|Random|RandomFloatinRange 0.0 6.28) (Math|Random|RandomFloat)) (|(vector((idx*100.000000),((r*percent)*(sin(angle))),((r*percent)*(cos(angle))))) _returnvalue_2 (|(((((((1.606200*x)*x)*x)-((28.084101*x)*x))+(211.432495*x))-184.921097)-((((0.033463*x)*x)*x)*x)) _returnvalue_2) (Math|Random|RandomFloatinRange 0.0 6.28) (Math|Random|RandomFloat)) (LocalVariables|GetbSpawnHealthP:ack) (LocalVariables|GetbSpawnEnemy)))))