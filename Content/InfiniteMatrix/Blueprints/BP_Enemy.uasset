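; BP_Enemy is an enemy actor in InfiniteMatrix that damages the player on contact or dies to projectiles.
; MeshCollision overlaps apply collision damage to BP_Player, displaying restart if DealDamage returns true, or destroy both enemy and BP_Projectile, awarding score.
; PassingCollision destroys the enemy once the player leaves that volume.
; Damage, reward and hit/kill counters go through GI_Instance, cached in the Construction Script.
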(event `self.MeshCollision.OnComponentBeginOverlap`
  (params (OverlappedComponent :type "PrimitiveComponent Object Reference") (OtherActor :type "Actor Object Reference") (OtherComp :type "PrimitiveComponent Object Reference") (OtherBodyIndex :type Integer) (bFromSweep :type Boolean) (SweepResult :type "HitResult Structure (by ref)"))
  (bind _gameinst (`self.GameInst`))
  (bind _gameinst_2 (`self.GameInst`))
  (bind _asbp_player (cast `/Game/InfiniteMatrix/Blueprints/BP_Player` OtherActor)
    (:`then`
      (bind _isdead (`/Game/InfiniteMatrix/Blueprints/BP_Player.DealDamage` _asbp_player (`/Game/InfiniteMatrix/Blueprints/GI_Instance.EnemyCollisionDamage` _gameinst)))
      (`/Game/InfiniteMatrix/Blueprints/GI_Instance.IncreaseCollidedEnemyCount` _gameinst)
      (if _isdead
        (`/Game/InfiniteMatrix/Blueprints/BP_Player.DisplayRestart` _asbp_player)))
    (:`CastFailed`
      (bind _asbp_projectile (cast `/Game/InfiniteMatrix/Blueprints/BP_Projectile` OtherActor))
      (`/Game/InfiniteMatrix/Blueprints/GI_Instance.AddScore` _gameinst_2 (`/Game/InfiniteMatrix/Blueprints/GI_Instance.KillEnemyReward` _gameinst_2))
      (`/Game/InfiniteMatrix/Blueprints/GI_Instance.IncreaseKilledEnemyCount` _gameinst_2)
      (`self.K2_DestroyActor`)
      (`self.K2_DestroyActor` _asbp_projectile))))

(event `self.PassingCollision.OnComponentEndOverlap`
  (params (OverlappedComponent :type "PrimitiveComponent Object Reference") (OtherActor :type "Actor Object Reference") (OtherComp :type "PrimitiveComponent Object Reference") (OtherBodyIndex :type Integer))
  (cast `/Game/InfiniteMatrix/Blueprints/BP_Player` OtherActor)
  (`self.K2_DestroyActor`))

(fn `UserConstructionScript`
  (bind _asgi_instance (cast `/Game/InfiniteMatrix/Blueprints/GI_Instance` (`GameplayStatics.GetGameInstance`)))
  (set `self.GameInst` _asgi_instance))