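; BP_Projectile is a short-lived projectile actor that flies along the world X axis and destroys itself after about one second.
; Tick accumulates elapsed time and applies a swept world offset from ForwardSpeed, scaled by the ProjectileSpeedUpFactor on GI_Instance.
; InitForwardSpeed sets the base speed from a speed and factor, and the construction script caches the game instance.
; The file contains no hit, overlap or damage handling.
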(event `self.ReceiveTick`
  (params (DeltaSeconds :type "Float (single-precision)"))
  (bind _output_get (set `self.TimePast` (+ DeltaSeconds (`self.TimePast`))))
  (if (> _output_get 1.0)
    (`self.K2_DestroyActor`)
    (else
      (`self.K2_AddActorWorldOffset` (`KismetMathLibrary.MakeVector` (* DeltaSeconds (`self.ForwardSpeed`) (`/Game/InfiniteMatrix/Blueprints/GI_Instance.ProjectileSpeedUpFactor` (`self.GameInst`)))) true))))

(fn `InitForwardSpeed`
  (params (Speed :type "Float (double-precision)") (Factor :type "Float (double-precision)"))
  (set `self.ForwardSpeed` (* Speed Factor)))

(fn `UserConstructionScript`
  (bind _asgi_instance (cast `/Game/InfiniteMatrix/Blueprints/GI_Instance` (`GameplayStatics.GetGameInstance`)))
  (set `self.GameInst` _asgi_instance))